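; Player bird character for a flying game, also handling start screen, player UI, score and game over on Wall overlap.
; Tick drives forward hops when grounded and, when airborne with wings open, forward velocity scaled by a decaying Boost, which braking drains faster.
; Dives close the wings and raise gravity; ending one converts fall speed into Boost.
; Hoop boosts and fast dive exits add extra Boost, while Leap launches the bird upward.
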(event `self.ReceiveBeginPlay`
  (bind _returnvalue (`|CreateWidget` "/Game/System/StartScreen.StartScreen_C"))
  (`UserWidget.AddToViewport` _returnvalue 0)
  (`GameplayStatics.SetGamePaused` true))

(event `StartGame`
  (`Widget.RemoveFromParent` (stale `self.ReceiveBeginPlay` _returnvalue))
  (bind _returnvalue (`|CreateWidget` "/Game/System/PlayerUI.PlayerUI_C"))
  (`UserWidget.AddToPlayerScreen` _returnvalue 0)
  (set `self.playerUI` _returnvalue)
  (set `self.hasStarted` true)
  (`GameplayStatics.SetGamePaused` false))

(event `self.ReceiveTick`
  (params (DeltaSeconds :type "Float (single-precision)"))
  (if (`self.struckWall`)
    _
    (elif (`NavMovementComponent.IsFalling` (`self.CharacterMovement`))
      (if (not (`self.wingsClosed`))
        (`self.forwardFlight`))
      (`self.slowDown`)
      (else
        (`self.forwardHop`)))))

(event `EndBoost`
  (`KismetSystemLibrary.Delay` 0.7)
  (set `self.isBoosting` false))

(event `EndLeap`
  (`KismetSystemLibrary.Delay` 0.7)
  (set `self.isLeaping` false))

(event `self.Box.OnComponentBeginOverlap`
  (params (OverlappedComponent :type "PrimitiveComponent Object Reference") (OtherActor :type "Actor Object Reference") (OtherComp :type "PrimitiveComponent Object Reference") (OtherBodyIndex :type Integer) (bFromSweep :type Boolean) (SweepResult :type "HitResult Structure (by ref)"))
  (cast `/Game/Models/Walls/Wall` OtherActor)
  (`self.hitWall`)
  (`KismetSystemLibrary.Delay` 0.3)
  (`self.loseGame`))

(fn `collectPoint`
  (set `self.score` (+ (`self.score`) 1)))

(fn `endDive`
  (if (and (`self.wingsClosed`) (not (`self.isLeaping`)))
    (set `self.wingsClosed` false)
    (set `CharacterMovementComponent.bOrientRotationToMovement` false (`self.CharacterMovement`))
    (set `self.bUseControllerRotationPitch` true)
    (set `self.boost` (/ (.z (`self.GetVelocity`)) -500.0))
    (if (>= (`self.boost`) 3.0)
      (`self.triggerBoost`))))

(fn `forwardFlight`
  (if (not (`self.isLeaping`))
    (set `MovementComponent.Velocity` (* (* (`KismetMathLibrary.GetForwardVector` (`self.K2_GetActorRotation`)) 600.0) (`self.boost`)) (`self.CharacterMovement`))))

(fn `forwardHop`
  (`self.AddMovementInput` (`KismetMathLibrary.GetForwardVector` (`self.K2_GetActorRotation`))))

(fn `hitWall`
  (bind _charactermovement (`self.CharacterMovement`))
  (set `self.struckWall` true)
  (set `MovementComponent.Velocity` (0.0 0.0 0.0) _charactermovement)
  (set `CharacterMovementComponent.GravityScale` 0.0 _charactermovement)
  (`GameplayStatics.PlaySound2D` "/Game/Sounds/zapsplat_horror_joint_rip_tear_break_003.zapsplat_horror_joint_rip_tear_break_003"))

(fn `hoopBoost`
  (if (<= (`self.boost`) (`self.maxBoost`))
    (set `self.isBraking` false)
    (if (not (`self.wingsClosed`))
      (`self.triggerBoost`))))

(fn `leap`
  (set `self.isLeaping` true)
  (`self.LaunchCharacter` (0.0 0.0 1700.0) true true)
  (`self.EndLeap`))

(fn `loseGame`
  (`GameplayStatics.SetGamePaused` true)
  (set `self.gameEnded` true)
  (`Widget.RemoveFromParent` (`self.playerUI`))
  (bind _returnvalue (`|CreateWidget` "/Game/System/LoseScreen.LoseScreen_C"))
  (`UserWidget.AddToViewport` _returnvalue 0))

(fn `slowDown`
  (bind _boost (`self.boost`))
  (if (> (`self.boost`) 1.0)
    (if (`self.isBraking`)
      (set `self.boost` (- _boost 0.07))
      (if (< _boost 1.0)
        (set `self.boost` 1.0))
      (else
        (set `self.boost` (- (`self.boost`) 0.01))))))

(fn `startDive`
  (bind _charactermovement (`self.CharacterMovement`))
  (if (<= (`self.boost`) 5.0)
    (set `self.wingsClosed` true)
    (set `CharacterMovementComponent.bOrientRotationToMovement` true (`self.CharacterMovement`))
    (set `self.bUseControllerRotationPitch` false)
    (set `CharacterMovementComponent.GravityScale` 2.0 _charactermovement)
    (set `MovementComponent.Velocity` (0.0 0.0 0.0) _charactermovement)))

(fn `triggerBoost`
  (set `self.boost` (+ (`self.boost`) 1.5))
  (set `self.isBoosting` false)
  (set `self.isBoosting` true)
  (`GameplayStatics.PlaySound2D` "/Game/Sounds/zapsplat_foley_rope_or_cable_whip_swish_through_ai.zapsplat_foley_rope_or_cable_whip_swish_through_ai" 0.3)
  (`self.EndBoost`))

(fn `UserConstructionScript`)